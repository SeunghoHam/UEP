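; BP_AnbyWeapon is Anby's weapon actor, wrapping a weapon mesh that fades in and out through a material effect.
; Show and Hide run timelines that drive the materials' "Phase" scalar, with visibility enabled before showing and disabled after hiding finishes.
; A view-state function instantly hides the mesh in first-person sight and shows it in third-person.
; HideWeapon forwards to Hide, while ShowWeapon is empty.
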(event EventShow
  (Rendering|SetVisibility (Variables|Default|GetWeaponMesh) true false)
  (bind _value (Timeline|ShowTL PlayFromStart)
    (:Update
      (Rendering|Material|SetScalarParameterValueonMaterials (Variables|Default|GetWeaponMesh) "Phase" (Math|Float|Lerp 0.0 1.2 _value)))))

(event EventHide
  (bind _value (Timeline|HideTL PlayFromStart)
    (:Update
      (Rendering|Material|SetScalarParameterValueonMaterials (Variables|Default|GetWeaponMesh) "Phase" (Math|Float|Lerp 1.0 0.0 _value)))
    (:Finished
      (Rendering|SetVisibility (Variables|Default|GetWeaponMesh) false false))))

(fn ConstructionScript)

(fn ChangeWeaponShowwithViewState
  (params (ViewState :type E_ViewState%20Enum :default "NewEnumerator0"))
  (bind _weaponmesh (Variables|Default|GetWeaponMesh))
  (switch Utilities|FlowControl|Switch|SwitchonE_ViewState ViewState
    (:NewEnumerator0
      (Rendering|SetVisibility _weaponmesh false false))
    (:NewEnumerator1
      (Rendering|SetVisibility _weaponmesh true false))))

(fn ShowWeapon)

(fn HideWeapon
  (Class|AnbyWeapon|Hide))

(fn GetWeaponStaticMesh
  (return (Variables|Default|GetWeaponMesh)))