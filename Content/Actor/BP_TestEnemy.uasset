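; BP_TestEnemy is a test melee enemy character that spawns a sword onto its hand socket on BeginPlay.
; Attack plays a montage and fires OnAttackEnd when it finishes or is interrupted, alongside knockdown and recursive chase-then-attack events.
; Helper functions expose combat ranges, patrol route and walk-speed tiers to AI.
; Each Tick updates a camera-facing 3D widget with HP, which also shows target marks.
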(event Custom|ChasePlayer
  (AI|AIMoveTo self "0, 0, 0" (Game|GetPlayerCharacter 0) 5.0 false
    (:OnSuccess
      (CallFunction|Attack)
      (Utilities|FlowControl|Delay 2.0)
      ;[1 1 1] 재귀함수
      (CallFunction|ChasePlayer))))

(event Custom|Attack
  (Animation|Montage|PlayMontage (Variables|Character|GetMesh) "/Game/Model/NewAnim/Attack/EnemyAttack_Montage.EnemyAttack_Montage"
    (:OnCompleted
      _)
    (:OnInterrupted
      _))
  ;[1 1 1] 좌측의 Event Dispatchers 에서 만듬
  ; 그리고 CAll
  (Default|CallOnAttackEnd))

(event Custom|WieldSword
  (bind _returnvalue (Game|SpawnActorfromClass "/Game/Actor/BP_AnbyWeapon.BP_AnbyWeapon_C" (Transformation|GetActorTransform) "Undefined" "MultiplyWithRoot" 0 0))
  (Transformation|AttachComponentToComponent _returnvalue (Variables|Character|GetMesh) "WeaponPoint" "SnapToTarget" "SnapToTarget" "SnapToTarget" true))

(event Custom|SetTarget
  (Development|PrintString "AI : SetTarget")
  (Variables|Default|SetIsSetTarget true))

(event Custom|AddMarking
  ;[1 1 1 1 40] Marking(Sword)
  (Default|AddTargetMark (Variables|Default|GetWBP_3DUI)))

(event Custom|RemoveMarking
  (params (NewParam :type Boolean))
  ;[1 1 1 1 40] Marking(Sword)
)

(event Custom|DownMontage
  (Animation|Montage|PlayMontage (Variables|Character|GetMesh) "/Game/Model/NewAnim/HitandDown/KnockDownNinjaKnockdownBack_Montage.KnockDownNinjaKnockdownBack_Montage"))

(event Custom|TestAttack_1
  (Animation|Montage|PlayMontage (Variables|Character|GetMesh) "/Game/Model/NewAnim/Attack/EnemyAttack_Montage.EnemyAttack_Montage"))

(event EventBeginPlay
  (CallFunction|WieldSword)
  (bind _aswbp_3dui (Utilities|Casting|CastToWBP_3DUI (UserInterface|GetUserWidgetObject (Variables|Default|Get3DUI))))
  (Variables|Default|SetWBP_3DUI _aswbp_3dui))

(event EventTick
  (params (DeltaSeconds :type Float%20%28single-precision%29))
  (CallFunction|Set3DUI))

(event Game|Damage|EventAnyDamage
  (params (Damage :type Float%20%28single-precision%29) (DamageType :type Damage%20Type%20Object%20Reference) (InstigatedBy :type Controller%20Object%20Reference) (DamageCauser :type Actor%20Object%20Reference)))

(fn ConstructionScript)

(fn Targeting
  (return false))

(fn Set3DUI
  (bind _wbp_3dui (Variables|Default|GetWBP_3DUI))
  (bind _3dui (Variables|Default|Get3DUI))
  (Utilities|IsValid _wbp_3dui
    (:Is%20Valid
      (Progress|SetPercent (Variables|/Game/Actor/WBP/WBP_3DUI.WBP_3DUI_C|GetHP_Bar _wbp_3dui) (Variables|/Game/Actor/Component/AC_EnemyStatus.AC_EnemyStatus_C|GetCurentHP (Variables|Default|GetAC_Status)))
      (Transformation|SetWorldRotation _3dui (Math|Rotator|FindLookatRotation (Transformation|GetWorldLocation _3dui) (Transformation|GetWorldLocation (Variables|/Script/Engine.Actor|GetRootComponent (Game|GetPlayerCameraManager 0)))) false false))))

(fn GetEnemyForward
  (return (Math|Vector|Normalize (Transformation|GetActorForwardVector))))

(fn GetIdealRange
  (return 1.5e+02 3.5e+02))

(fn GetPatrolRoute
  (return (Variables|AI|GetPatrolRoute)))

(fn SetMovementSpeed
  (params (Speed :type E_MovementSpeed%20Enum :default "NewEnumerator0"))
  (bind _output_get (Variables|/Script/Engine.CharacterMovementComponent|SetMaxWalkSpeed (Variables|Character|GetCharacterMovement) (Utilities|Select :Index Speed :NewEnumerator0 0.0 :NewEnumerator1 2e+02 :NewEnumerator2 3e+02 :NewEnumerator3 5e+02)))
  (return _output_get))