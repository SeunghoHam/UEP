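; AC_EnemyStatus is an actor component that holds an enemy's HP, MP and death state.
; On BeginPlay it casts its owner to BaseEnemy and caches it.
; SetDefaultState sets HP and MP, while CheckDead subtracts damage from HP and returns the remaining HP with a dead flag set at zero or below.
; GetCurrentHP exposes the current HP.
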(event EventBeginPlay
  (bind _asbase_enemy (Utilities|Casting|CastToBaseEnemy (Components|GetOwner)))
  (Variables|Default|SetBase%20Enemy _asbase_enemy))

(event EventTick
  (params (DeltaSeconds :type Float%20%28single-precision%29)))

(fn GetCurrentHP
  (return (Variables|Default|GetCurentHP)))

(fn CheckDead
  (params (Damage :type Float%20%28double-precision%29))
  (bind _output_get (Variables|Default|SetCurentHP (- (Variables|Default|GetCurentHP) Damage)))
  (if (<= _output_get 0.0)
    (Variables|Default|SetbIsDead true)
    (else
      (Variables|Default|SetbIsDead false)))
  (return (Variables|Default|GetbIsDead) _output_get))

(fn SetDefaultState
  (params (HP :type Float%20%28double-precision%29) (MP :type Integer))
  (Variables|Default|SetCurentHP HP)
  (Variables|Default|SetCurrentMP MP))