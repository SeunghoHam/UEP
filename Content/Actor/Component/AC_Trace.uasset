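; Melee hit-detection component for BP_Anby, apparently work in progress with damage and HP-bar updates disconnected.
; A looping timer sphere-traces between the sword's sockets, printing and casting the first Damageable hit behind a DoOnce whose reset is unwired.
; WeaponTrace box-traces from the previous socket position but ignores the result.
; DoAttack calls CheckCollisionRange, which plays shake and sound, box-traces forward and returns an Enemy-tagged actor, left unused.
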(event Custom|StopSwordTrace
  ;[1 1 1] SwordTRace
  (Utilities|Time|ClearandInvalidateTimerbyHandle (Variables|Default|GettSwordTraceLoop)))

(event Custom|StartSwordTrace
  ;[1 1 1] SwordTRace
  (bind _returnvalue (Utilities|Time|SetTimerbyEvent (delegate Custom|SwordTraceLoop) 0.001 true))
  (Variables|Default|SettSwordTraceLoop _returnvalue))

(event Custom|ChainAttack
  (params (Damage :type Float%20%28double-precision%29)))

(event Custom|SwordTraceLoop
  (bind _character (Variables|Default|GetCharacter))
  (bind _returnvalue (Class|Anby|GetAnbyWeapon _character))
  (bind _returnvalue_2 (Class|AnbyWeapon|GetMesh _returnvalue))
  ;[1 1 1] SwordTRace
  ;;[1 1 1] Visiblity 타입으로 때림,
  ;; 적 Block 으로설정해주기
  (bind (_outhit _returnvalue_3) (Collision|SphereTraceByChannel (Transformation|GetSocketLocation _returnvalue_2 "TopTrace") (Transformation|GetSocketLocation _returnvalue_2 "BottomTrace") 3e+01 "TraceTypeQuery1" false 0 "ForDuration" true "(R=1.000000,G=0.000000,B=0.000000,A=1.000000)" "(R=0.000000,G=1.000000,B=0.000000,A=1.000000)" 1.0))
  (if _returnvalue_3
    (if (Actor|ActorHasTag (.HitActor (Collision|BreakHitResult _outhit)) "Damageable")
      (Utilities|FlowControl|DoOnce false
        (:Completed
          (Development|PrintString (Utilities|GetDisplayName (.HitActor (Collision|BreakHitResult _outhit))))
          (bind _asbp_drake (Utilities|Casting|CastToBP_Drake (.HitActor (Collision|BreakHitResult _outhit)))))))))

(event Custom|SphereTrace
  ;[1 1 1] SphereTrace(Kick and Melee)
)

(event Custom|PlaySwordHitSounds
  (Audio|PlaySoundatLocation "/Game/Resource/Sound/MS_SwordHit.MS_SwordHit" (Transformation|GetActorLocation (Components|GetOwner)) "0, 0, 0" 1.0 1.0 0.0 0 0 0 0))

(event EventBeginPlay
  (bind _asbp_anby (Utilities|Casting|CastToBP_Anby (Components|GetOwner)))
  (Variables|Default|SetCharacter _asbp_anby)
  (Variables|Default|SetCharacterMesh (Variables|/Script/Engine.Character|GetMesh _asbp_anby)))

(fn WeaponTrace
  (bind _returnvalue (Components|GetOwner))
  (if (Variables|Default|GetbWeaponTrace)
    (bind _asbp_anby (Utilities|Casting|CastToBP_Anby _returnvalue)
      (:then
        (Development|PrintString "Anby Cast Success")
        (bind _weaponmesh (Class|BICombatComponent|GetWeaponStaticMesh(Message) _returnvalue))
        (LocalVariables|SetCurrentTopLocation (Transformation|GetSocketLocation _weaponmesh "TopTrace"))
        (LocalVariables|SetCurrentBottomLocation (Transformation|GetSocketLocation _weaponmesh "BottomTrace"))
        (Collision|BoxTraceByChannel (Variables|Default|GetPreviousTopSocket) (LocalVariables|GetCurrentBottomLocation) (Math|Vector|MakeVector (/ (Math|Vector|Distance(Vector) (LocalVariables|GetCurrentTopLocation) (LocalVariables|GetCurrentBottomLocation)) 2.0) 0.0 0.0) (Math|Rotator|FindLookatRotation (LocalVariables|GetCurrentTopLocation) (LocalVariables|GetCurrentBottomLocation)) "TraceTypeQuery1" false 0 "None")
        (Variables|Default|SetPreviousTopSocket (LocalVariables|GetCurrentTopLocation))
        (Variables|Default|SetPreviousBottomSocket (LocalVariables|GetCurrentBottomLocation)))
      (:CastFailed
        (Development|PrintString "Anby Cast Failed")))))

(fn CheckCollisionRange
  (params (HalfSize :type Vector :default "50.000000,50.000000,25.000000") (Start :type Float%20%28double-precision%29) (End :type Float%20%28double-precision%29))
  (bind _returnvalue (Components|GetOwner))
  (bind _returnvalue_2 (Transformation|GetActorLocation _returnvalue))
  (bind _returnvalue_3 (Transformation|GetActorForwardVector _returnvalue))
  (bind (_outhits _returnvalue_4) (Class|KismetSystemLibrary|BoxTraceMulti (+ _returnvalue_2 (* _returnvalue_3 Start)) (+ _returnvalue_2 (* _returnvalue_3 End)) HalfSize (Transformation|GetActorRotation _returnvalue) "TraceTypeQuery1" false 0 "ForDuration" true "(R=1.000000,G=0.000000,B=0.000000,A=1.000000)" "(R=0.000000,G=1.000000,B=0.000000,A=1.000000)" 0.5))
  (Camera|PlayWorldCameraShake "/Game/Actor/BP_HitCameraShake.BP_HitCameraShake_C" (Transformation|GetActorLocation (Components|GetOwner)) 0.0 2e+03)
  (CallFunction|PlaySwordHitSounds)
  (if _returnvalue_4
    (for _array_element _outhits
      (if (Actor|ActorHasTag (.HitActor (Collision|BreakHitResult _array_element)) "Enemy")
        (return (.HitActor (Collision|BreakHitResult _array_element)))
        (else
          (Development|PrintString "맞은아이가 없으셈"))))))

(fn DoAttack
  (params (Damage :type Float%20%28double-precision%29) (HalfSize :type Vector :default "50.000000,50.000000,25.000000") (Start :type Float%20%28double-precision%29) (End :type Float%20%28double-precision%29))
  (bind _isactor (CallFunction|CheckCollisionRange HalfSize Start End))
  (Utilities|IsValid _isactor))

(fn GetWeaponStaticMesh
  (return 0))