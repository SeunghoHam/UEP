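; Enemy attack component, still a prototype, that checks whether a melee slash reaches the player.
; SlashAttack calls CheckCollisionRange, which runs a debug-drawn multi box trace on the Visibility channel along the owner's forward vector.
; A Player-tagged hit passes a DoOnce, prints a message and casts to BP_Anby, with no damage applied.
; TurnAttack is an empty stub, and the owner-rotation logic in the event graph is unconnected.
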(event EventBeginPlay)

(event EventTick
  (params (DeltaSeconds :type Float%20%28single-precision%29)))

(fn SlashAttack
  (Development|PrintString "StartAttack")
  (CallFunction|CheckCollisionRange "100.000000,100.000000,50.000000" 5e+01 1.5e+02))

(fn TurnAttack)

(fn CheckCollisionRange
  (params (HalfSize :type Vector :default "100.000000,100.000000,50.000000") (Start :type Float%20%28double-precision%29) (End :type Float%20%28double-precision%29))
  (bind _returnvalue (Components|GetOwner))
  (bind _returnvalue_2 (Transformation|GetActorForwardVector _returnvalue))
  (bind _returnvalue_3 (Transformation|GetActorLocation _returnvalue))
  ;[1 1 1] halfsize = 박스 각 축의 절반 길이
  (bind (_outhits _returnvalue_4) (Class|KismetSystemLibrary|BoxTraceMulti (+ _returnvalue_3 (* _returnvalue_2 Start)) (+ _returnvalue_3 (* _returnvalue_2 End)) HalfSize (Transformation|GetActorRotation _returnvalue) "TraceTypeQuery1" false 0 "ForDuration" true "(R=1.000000,G=1.000000,B=1.000000,A=1.000000)" "(R=1.000000,G=0.032176,B=0.000000,A=1.000000)" 0.5))
  (if _returnvalue_4
    (for _array_element _outhits
      (if (Actor|ActorHasTag (.HitActor (Collision|BreakHitResult _array_element)) "Player")
        (Utilities|FlowControl|DoOnce false
          (:Completed
            (Development|PrintString "딱걸렸다잇")
            (Utilities|Casting|CastToBP_Anby (.HitActor (Collision|BreakHitResult _array_element)))))))))