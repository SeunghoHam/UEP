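; Camera component for the BP_Anby character that handles switching between first and third person views.
; BeginPlay caches the owner's spring arm and camera and prints debug checks on both.
; ChangeCharacterViewType toggles the view type, mesh option and controller-yaw rotation.
; PrevSetting picks the target arm length for the opposite view, and SetSpringArmLength blends the character's base arm length toward it using an Alpha supplied by the caller.
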(event EventBeginPlay
  (bind _asbp_anby (Utilities|Casting|CastToBP_Anby (Components|GetOwner)))
  (Variables|Components|SetCharacter _asbp_anby)
  (Variables|Default|SetSpringArmComponent (Variables|/Script/WorkTest.Anby|GetSpringArmComponent _asbp_anby))
  (Variables|Default|SetCamera%20Component (Variables|/Script/WorkTest.Anby|GetCameraComponent _asbp_anby))
  (Utilities|FlowControl|Sequence
    (:then_0
      (Utilities|IsValid (Variables|Default|GetCamera%20Component)
        (:Is%20Valid
          (Development|PrintString "AC_CameraSystem : Camera ON" true true "(R=1.000000,G=1.000000,B=1.000000,A=1.000000)" 3.0))
        (:Is%20Not%20Valid
          (Development|PrintString "AC_CameraSystem : Camera OFF" true true "(R=1.000000,G=0.000000,B=0.000000,A=1.000000)" 3.0))))
    (:then_1
      (Utilities|IsValid (Variables|Default|GetSpringArmComponent)
        (:Is%20Valid
          (Development|PrintString "AC_CameraSystem : SpringArm On" true true "(R=1.000000,G=1.000000,B=1.000000,A=1.000000)" 3.0))
        (:Is%20Not%20Valid
          (Development|PrintString "AC_CameraSystem : SpringArm OFF" true true "(R=1.000000,G=0.000000,B=0.000000,A=1.000000)" 3.0))))))

(event EventTick
  (params (DeltaSeconds :type Float%20%28single-precision%29)))

(fn ChangeCharacterViewType
  (bind _character (Variables|Components|GetCharacter))
  ;[1 1 1] 현재 상태
  (switch Utilities|FlowControl|Switch|SwitchonEViewType (Class|Anby|GetViewType (Variables|Components|GetCharacter))
    (:ThirdSight
      (Default|SetMeshOption _character false)
      ;[1 1 1] 3인칭 - 1인칭 전환
      (Variables|/Script/Engine.Pawn|SetbUseControllerRotationYaw _character true)
      (Class|Anby|ChangeViewType _character (LocalVariables|GetFirstView)))
    (:FirstSight
      (Default|SetMeshOption _character true)
      (Variables|/Script/Engine.Pawn|SetbUseControllerRotationYaw _character false)
      (Class|Anby|ChangeViewType _character (LocalVariables|GetThirdView)))))

(fn SetSpringArmLength
  (params (alpha :type Float%20%28double-precision%29))
  (Class|Anby|SetBaseTargetArmLength (Variables|Components|GetCharacter) (Math|Float|Lerp (Variables|Default|GetCurrentSpringArmLenght) (Variables|Default|GetTargetSpringArmLegnth) alpha)))

(fn PrevSetting
  (params (Current :type Float%20%28double-precision%29))
  (Variables|Default|SetCurrentSpringArmLenght Current)
  (switch Utilities|FlowControl|Switch|SwitchonEViewType (Class|Anby|GetViewType (Variables|Components|GetCharacter))
    (:ThirdSight
      (Variables|Default|SetTargetSpringArmLegnth 0.0)
      (Development|PrintString "0 Setting"))
    (:FirstSight
      (Variables|Default|SetTargetSpringArmLegnth 3e+02)
      (Development|PrintString "300 Setting"))))