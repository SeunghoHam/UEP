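; AC_Grapple is a prototype grappling-hook component for BP_Anby, apparently cable-based, driven externally since Tick is empty.
; ShootGrapple traces along the view to store attach and move points; SpawnGrappleHook places the hook actor.
; Move functions switch the owner's MovementState and gravity, pulling it toward the point by tension or shift-held interpolation.
; GrappleLengthLimit constrains rope length, CancelMove restores Ground, and debug prints, traces and disconnected experiments remain.
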(event EventBeginPlay
  (bind _asbp_anby (Utilities|Casting|CastToBP_Anby (Components|GetOwner)))
  (bind _output_get (Variables|Default|SetOwner _asbp_anby))
  (bind _asplayer_controller (Utilities|Casting|CastToPlayerController (Pawn|GetController _output_get)))
  (Variables|Default|SetPlayer%20Controller _asplayer_controller)
  (Variables|/Script/WorkTest.Anby|SetMovementState (Variables|Default|GetOwner) "Ground"))

(event EventTick
  (params (DeltaSeconds :type Float%20%28single-precision%29)))

(fn InitGrapple
  ;[1 1 1] 초기화
)

(fn ShootGrapple
  (bind _returnvalue (Viewport|GetViewportSize))
  (bind _player_controller (Variables|Default|GetPlayer%20Controller))
  (bind (_x _y) (Math|Vector2D|BreakVector2D _returnvalue))
  (bind _returnvalue_2 (/ _x 2.0))
  (bind _returnvalue_3 (/ _y 2.0))
  (bind (_worldposition _worlddirection) (Class|GameplayStatics|DeprojectScreentoWorld _player_controller (Math|Vector2D|MakeVector2D _returnvalue_2 _returnvalue_3)))
  (if (Utilities|Enum|Equal(Enum) (Variables|/Script/WorkTest.Anby|GetMovementState (Variables|Default|GetOwner)) "Ground")
    ;[1 1 1] 초기화 테스트
    (Variables|Default|SetForce "0, 0, 0")
    (Variables|Default|SetVelocity "0, 0, 0")
    (LocalVariables|SetWorldLocation _worldposition)
    (LocalVariables|SetWorldDirection _worlddirection)
    (Variables|GrappleMove|SetGrapple_StartPoint (Transformation|GetActorLocation (Variables|Default|GetOwner)))
    (bind (_outhit _returnvalue_4) (Collision|LineTraceByChannel (Variables|GrappleMove|GetGrapple_StartPoint) (+ (Variables|GrappleMove|GetGrapple_StartPoint) (* (.Rotation (Pawn|GetPlayerViewPoint (Variables|Default|GetPlayer%20Controller))) 5e+03)) "TraceTypeQuery1" false 0 "None" true "(R=1.000000,G=1.000000,B=1.000000,A=1.000000)"))
    (Variables|Default|SetbIsHit _returnvalue_4)
    (if _returnvalue_4
      (CallFunction|DeleteGarppleActor)
      (bind _output_get (Variables|GrappleMove|SetGrapple_AttachPoint (+ (.ImpactPoint (Collision|BreakHitResult _outhit)) (* (.ImpactNormal (Collision|BreakHitResult _outhit)) 5.0))))
      (Variables|GrappleMove|SetGrapple_MovePoint (+ (.ImpactPoint (Collision|BreakHitResult _outhit)) (* (.ImpactNormal (Collision|BreakHitResult _outhit)) 25.0)))
      (Variables|GrappleMove|SetToGrappleDirection (Math|Vector|Normalize (- _output_get (Variables|GrappleMove|GetGrapple_StartPoint)))))))

(fn DeleteGarppleActor
  (Utilities|IsValid (Variables|Grapple|GetGrappleActor)
    (:Is%20Valid
      (Actor|DestroyActor (Variables|Grapple|GetGrappleActor))
      (Variables|Grapple|SetGrappleActor 0)
      (Variables|Default|SetbIsHookPin false))))

(fn GrappleMovewithVelocity
  (params (DeltaTime :type Float%20%28double-precision%29))
  (bind _grapple_movepoint (Variables|GrappleMove|GetGrapple_MovePoint))
  (bind _owner (Variables|Default|GetOwner))
  (bind _returnvalue (Transformation|GetActorLocation _owner))
  ;[1 1 1] 수치대로 이동시키기 테스트
  (CallFunction|CheckMoveTrace)
  (switch Utilities|FlowControl|Switch|SwitchonEMovementState (Variables|/Script/WorkTest.Anby|GetMovementState (Variables|Default|GetOwner))
    (:Moving
      (bind _output_get (LocalVariables|SetDirection (Math|Vector|Normalize (- _grapple_movepoint _returnvalue))))
      (Variables|Default|SetDistance (Math|Vector|Distance(Vector) _grapple_movepoint _returnvalue))
      (bind _output_get_2 (Variables|Default|SetForce (* _output_get (Variables|Default|GetTension))))
      (bind _output_get_3 (Variables|Default|SetVelocity (+ (* (+ _output_get_2 (LocalVariables|GetGravity)) DeltaTime) (Transformation|GetActorLocation _owner))))
      (Transformation|SetActorLocation _owner (+ "" _output_get_3) true false)
      (if (<= (Variables|Default|GetDistance) 1e+02)
        (CallFunction|ReachMovePoint)))
    (:Falling
      (Transformation|SetActorLocation (Variables|Default|GetOwner) (+ (* (+ (* (Variables|GrappleMove|GetToGrappleDirection) (/ (Variables|Default|GetTension) 2.0)) (LocalVariables|GetGravity)) DeltaTime) (Transformation|GetActorLocation (Variables|Default|GetOwner))) true false))))

(fn OrderGrappleMove
  (if (Variables|Default|GetbIsHit)
    (Variables|Default|SetbIsHit false)
    (if (Variables|Default|GetbIsGrappling)
      (Development|PrintString "IsGrapping= true" true true "(R=0.121427,G=1.000000,B=0.000000,A=1.000000)" 1.0)
      (else
        (Development|PrintString "IsGrapping = false" true true "(R=0.000773,G=1.000000,B=0.000000,A=1.000000)" 1.0)))
    (Utilities|IsValid (Variables|Grapple|GetGrappleActor)
      (:Is%20Valid
        (Variables|/Script/WorkTest.Anby|SetMovementState (Variables|Default|GetOwner) "Moving")
        (Variables|Default|SetbIsMoveInRange false)
        (CallFunction|EnableGravity false)
        (Character|LaunchCharacter (Variables|Default|GetOwner) "0.000000,0.000000,200.000000" false false)
        (Variables|Default|SetbIsGrappling true)))))

(fn SpawnGrappleHook
  (params (HitActorRotation :type Rotator))
  (bind _returnvalue (Game|SpawnActorfromClass "/Game/Actor/BP_GrapplePointActor.BP_GrapplePointActor_C" (Math|Conversions|ToTransform(Vector) (Variables|GrappleMove|GetGrapple_AttachPoint)) "Undefined" "MultiplyWithRoot" 0 0))
  (bind _output_get (Variables|Grapple|SetGrappleActor _returnvalue))
  (Transformation|SetActorRotation _output_get (Math|Conversions|RotationFromXVector (Math|Vector|Normalize (- (Transformation|GetActorLocation _output_get) (Transformation|GetActorLocation (Variables|Default|GetOwner))))))
  (Variables|Default|SetbIsHookPin true))

(fn GrappleLengthLimit
  (bind _grapple_movepoint (Variables|GrappleMove|GetGrapple_MovePoint))
  (if (Variables|Default|GetbIsGrappling)
    (bind _output_get (Variables|GrappleMove|SetCurrentGrappleLength (Math|Vector|Distance(Vector) (Transformation|GetActorLocation (Variables|Default|GetOwner)) (Variables|GrappleMove|GetGrapple_AttachPoint))))
    (if (> _output_get (Variables|GrappleMove|GetMaxGrappleLength))
      (Class|Anby|ServerMoveCharacter (Variables|Default|GetOwner) (- _grapple_movepoint (* (Math|Vector|Normalize (- _grapple_movepoint (Transformation|GetActorLocation (Variables|Default|GetOwner)))) (Variables|GrappleMove|GetMaxGrappleLength)))))))

(fn GrappleAdjustForce
  ;[1 1 1] 등속도운동 구현하기
)

(fn ReachMovePoint
  ;[1 1 1] 이동 종료
  (if (Utilities|Enum|Equal(Enum) "Moving" (Variables|/Script/WorkTest.Anby|GetMovementState (Variables|Default|GetOwner)))
    (Development|PrintString "Reach Move Point" true true "(R=1.000000,G=0.098677,B=0.000000,A=1.000000)")
    ;[1 1 1] 공중에서 와이어로 버티고 있는상태
    (Variables|/Script/WorkTest.Anby|SetMovementState (Variables|Default|GetOwner) "Grappling")
    (CallFunction|EnableGravity false)
    (else
      (Development|PrintString "Reach- false"))))

(fn CancelMove
  ;[1 1 1] 그래플링을 해제하면서 기억한 방향대로 계속 이동
  (Variables|Default|SetbIsGrappling false)
  (Variables|Shift|SetbIsShift false)
  (switch Utilities|FlowControl|Switch|SwitchonEMovementState (Variables|/Script/WorkTest.Anby|GetMovementState (Variables|Default|GetOwner))
    (:Hook
      _)
    (:Moving
      _)
    (:Grappling
      _))
  (CallFunction|ResetGrappleOption)
  (CallFunction|CheckSidewithCancel))

(fn ResetGrappleOption
  (Variables|/Script/WorkTest.Anby|SetMovementState (Variables|Default|GetOwner) "Ground")
  (Development|PrintString "Reset Grapple" true true "(R=1.000000,G=0.873644,B=0.000000,A=1.000000)" 1.0)
  (CallFunction|EnableGravity true))

(fn CheckMoveTrace
  (bind _owner (Variables|Default|GetOwner))
  (bind _returnvalue (Transformation|GetActorLocation _owner))
  (bind (_outhit _returnvalue_2) (Collision|LineTraceByChannel _returnvalue (+ _returnvalue (* (Transformation|GetActorForwardVector _owner) (Variables|Default|GetInMoveCheckDistance))) "TraceTypeQuery1" false 0 "ForDuration" true "(R=1.000000,G=1.000000,B=1.000000,A=1.000000)" "(R=1.000000,G=0.000000,B=0.580762,A=1.000000)" 1.0))
  (if _returnvalue_2
    (Rendering|Debug|DrawDebugSphere (.ImpactPoint (Collision|BreakHitResult _outhit)) 64.0 12 "(R=1.000000,G=0.000000,B=0.035748,A=1.000000)" 1.0)
    ;[1 1 1] 이 상태에서 C 누르면 위로 뽕
    (Variables|Default|SetbIsMoveInRange true)))

(fn EnableGravity
  (params (Enable :type Boolean))
  (bind _owner (Variables|Default|GetOwner))
  (if Enable
    (Physics|SetEnableGravity (Variables|/Script/Engine.Character|GetMesh _owner) true)
    (Variables|/Script/Engine.CharacterMovementComponent|SetGravityScale (Variables|/Script/Engine.Character|GetCharacterMovement _owner) 1.5)
    (else
      (Variables|/Script/Engine.CharacterMovementComponent|SetGravityScale (Variables|/Script/Engine.Character|GetCharacterMovement (Variables|Default|GetOwner)) 0.0)
      (Physics|SetEnableGravity (Variables|/Script/Engine.Character|GetMesh (Variables|Default|GetOwner)) false))))

(fn InputDirection
  (bind _owner (Variables|Default|GetOwner))
  (bind _owner_2 (Variables|Default|GetOwner))
  (bind _value (Default|GetDirection _owner))
  (Variables|Direction|SetFrontBack (.x _value))
  (Variables|Direction|SetRightLeft (.y _value))
  (return (* (+ (* (Transformation|GetActorRightVector _owner_2) (Variables|Direction|GetRightLeft)) (* (Transformation|GetActorUpVector _owner_2) (Variables|Direction|GetFrontBack))) 1e+01)))

(fn ShiftStart
  (bind _owner (Variables|Default|GetOwner))
  ;[1 1 1] 현재 Move or Grapple 상태인지 확인 후
  (switch Utilities|FlowControl|Switch|SwitchonEMovementState (Variables|/Script/WorkTest.Anby|GetMovementState _owner)
    (:Hook
      _)
    (:Grappling
      _))
  (Variables|Shift|SetbIsShift true)
  (Variables|/Script/WorkTest.Anby|SetMovementState _owner "Moving")
  (CallFunction|EnableGravity false))

(fn ShiftEnd
  (switch Utilities|FlowControl|Switch|SwitchonEMovementState (Variables|/Script/WorkTest.Anby|GetMovementState (Variables|Default|GetOwner))
    (:Hook
      _)
    (:Moving
      _))
  (Variables|Shift|SetbIsShift false)
  (if (CallFunction|LeftDistanceCheck)
    (Variables|Default|SetbIsGrappling true)
    (Variables|/Script/WorkTest.Anby|SetMovementState (Variables|Default|GetOwner) "Grappling")
    (CallFunction|EnableGravity true)
    (else
      (Variables|/Script/WorkTest.Anby|SetMovementState (Variables|Default|GetOwner) "Ground")
      (CallFunction|EnableGravity true))))

(fn CheckShift
  (params (delta :type Float%20%28double-precision%29) (MoveSpeed :type Float%20%28double-precision%29))
  (bind _grapple_movepoint (Variables|GrappleMove|GetGrapple_MovePoint))
  (if (Variables|Shift|GetbIsShift)
    (switch Utilities|FlowControl|Switch|SwitchonEMovementState (Variables|/Script/WorkTest.Anby|GetMovementState (Variables|Default|GetOwner))
      (:Moving
        _)
      (:Grappling
        _))
    (Variables|Default|SetMoveAmount (+ (Variables|Default|GetMoveAmount) 0.0))
    (bind _output_get (LocalVariables|SetFinalVelocity (* (- _grapple_movepoint (Transformation|GetActorLocation (Variables|Default|GetOwner))) MoveSpeed)))
    (Class|Anby|ServerMoveCharacter (Variables|Default|GetOwner) (+ (Transformation|GetActorLocation (Variables|Default|GetOwner)) (Math|Interpolation|VInterpTo (Transformation|GetActorLocation (Variables|Default|GetOwner)) _grapple_movepoint delta MoveSpeed)))
    (else
      (CallFunction|GrappleLengthLimit))))

(fn CheckSidewithCancel
  (bind _owner (Variables|Default|GetOwner))
  (bind _returnvalue (Transformation|GetActorLocation _owner))
  (bind _returnvalue_2 (Collision|LineTraceByChannel _returnvalue (+ _returnvalue (* (.Rotation (Pawn|GetPlayerViewPoint (Variables|Default|GetPlayer%20Controller))) 1e+03)) "TraceTypeQuery1" false 0 "ForDuration" true "(R=1.000000,G=0.000000,B=0.042158,A=1.000000)" "(R=0.000000,G=1.000000,B=0.000000,A=1.000000)" 3.0))
  (if _returnvalue_2
    (return false)
    (else
      (return true))))

(fn LeftDistanceCheck
  ;[1 1 1] Shift이동하다가 남은 거리가 MaxGrappleLength
  (if (< (Math|Vector|Distance(Vector) (Variables|GrappleMove|GetGrapple_MovePoint) (Transformation|GetActorLocation (Variables|Default|GetOwner))) (Variables|GrappleMove|GetMaxGrappleLength))
    (Development|PrintString "Grappling으로 전환" true true "(R=0.000000,G=0.660000,B=1.000000,A=1.000000)" 1.0)
    (return true)
    (else
      (Development|PrintString "그냥 멈추기" true true "(R=0.000000,G=0.660000,B=1.000000,A=1.000000)" 1.0)
      (return false))))