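; BP_Drake is an AI-controlled melee enemy character with health, attack, knockdown and dead animations, and sword target marking.
; Attacks play a montage or set EnemyAnimInstance state, broadcasting their end through a dispatcher.
; ACEnemyStatus feeds damage results to a camera-facing 3D HP widget, but the death check is unwired.
; A timeline slerps quaternions toward the AI controller's target, while getters expose ranges, patrol route and speed presets.
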(event Custom|LookTarget
  (CallFunction|SetQuat)
  (bind _lookat (Timeline|lookat PlayFromStart)
    (:Update
      (CallFunction|SetActorRotation _lookat))))

(event Custom|SetTarget
  (Variables|Default|SetbIsSetTarget true))

(event Custom|DownMontgae
  (Animation|Montage|PlayMontage (Variables|Character|GetMesh) "/Game/Model/NewAnim/HitandDown/KnockDownNinjaKnockdownBack_Montage.KnockDownNinjaKnockdownBack_Montage"))

(event Custom|Attack
  (Development|PrintString "Attack")
  (Animation|Montage|PlayMontage (Variables|Character|GetMesh) "/Game/Model/EnemySM/Anim/RightCrossAttackNinjaRightCross_Montage.RightCrossAttackNinjaRightCross_Montage"
    (:OnCompleted
      _)
    (:OnInterrupted
      _))
  ;[1 1 1] 좌측의 EventDispatchers
  (Default|CallCallonAttackEnd))

(event Custom|AddMarking
  ;[1 1 1 1 40] Marking(Sword)
  (Default|AddTargetMark (Variables|Default|GetWBP%203DUI)))

(event Custom|RemoveMarking
  (params (NewParam :type Boolean))
  ;[1 1 1 1 40] Marking(Sword)
  (Default|RemoveTargetMark (Variables|Default|GetWBP%203DUI)))

(event EventBeginPlay
  (bind _aswbp_3dui (Utilities|Casting|CastToWBP_3DUI (UserInterface|GetUserWidgetObject (Variables|Default|GetWidget))))
  (Variables|Default|SetWBP%203DUI _aswbp_3dui)
  (bind _asenemy_anim_instance (Utilities|Casting|CastToEnemyAnimInstance (Components|SkeletalMesh|GetAnimInstance (Variables|Character|GetMesh))))
  (bind _output_get (Variables|Default|SetAnimInstance _asenemy_anim_instance))
  ;[1 1 1] 이거 되는거 맞음?
  (Class|AnimInstance|SetRootMotionMode _output_get "RootMotionFromMontagesOnly")
  (Default|SetDefaultState (Variables|Default|GetAC_EnemyStatus) 2e+01 10))

(event Collision|EventActorBeginOverlap
  (params (OtherActor :type Actor%20Object%20Reference)))

(event EventTick
  (params (DeltaSeconds :type Float%20%28single-precision%29))
  ;[1 1 1] 플레이어 시야로 위치변경 시켜야함
  (CallFunction|Set3DUI))

(event EventGetDamaged
  (params (damage :type Float%20%28single-precision%29))
  ;[1 1 1 1 25] BP 정의 ( Damaged, IsDead)
  (bind (_isdead _currenthp) (Default|CheckDead (Variables|Default|GetAC_EnemyStatus) damage))
  (Development|PrintString (Utilities|String|ToString(Float) _currenthp) true true "(R=0.000000,G=1.000000,B=0.056358,A=1.000000)")
  (Default|SetHPPercent (Variables|Default|GetWBP%203DUI) _currenthp)
  (Class|BaseEnemy|TestDamaged 1e+01))

(event EventIsDead
  ;[1 1 1 1 25] BP 정의 ( Damaged, IsDead)
  (Variables|/Script/WorkTest.EnemyAnimInstance|SetAnimState (Variables|Default|GetAnimInstance) "Dead"))

(fn ConstructionScript)

(fn Set3DUI
  (bind _widget (Variables|Default|GetWidget))
  (Utilities|IsValid (Variables|Default|GetWBP%203DUI)
    (:Is%20Valid
      (Transformation|SetWorldRotation _widget (Math|Rotator|FindLookatRotation (Transformation|GetWorldLocation _widget) (Transformation|GetWorldLocation (Variables|/Script/Engine.Actor|GetRootComponent (Game|GetPlayerCameraManager 0)))) false false))))

(fn AttackRightCross
  ;[1 1 1] BT에서 실행됨
  (Variables|/Script/WorkTest.EnemyAnimInstance|SetAnimState (Variables|Default|GetAnimInstance) "Attack"))

(fn AttackEnd
  (Variables|/Script/WorkTest.EnemyAnimInstance|SetAnimState (Variables|Default|GetAnimInstance) "Locomotion")
  (Default|CallCallonAttackEnd))

(fn SetActorRotation
  (params (alpha :type Float%20%28double-precision%29))
  (Transformation|SetActorRotation (Class|KismetMathLibrary|QuatRotator (Class|KismetMathLibrary|QuatSlerp (Variables|Default|GetPrevActorQuat) (Variables|Default|GetTargetQuat) alpha))))

(fn SetQuat
  (Variables|Default|SetPrevActorQuat (Math|Conversions|ToQuaternion(Rotator) (Transformation|GetActorRotation)))
  (bind _asaic_enemy_base (Utilities|Casting|CastToAIC_Enemy_Base (Pawn|GetController)))
  (Utilities|IsValid (Variables|/Game/Actor/AI/AIC_Enemy_Base.AIC_Enemy_Base_C|GetAttackTarget _asaic_enemy_base)
    (:Is%20Valid
      (Variables|Default|SetTargetQuat (Math|Conversions|ToQuaternion(Rotator) (Math|Rotator|GetRotationXVector (Math|Conversions|RotationFromXVector (Math|Vector|Normalize (- (Transformation|GetActorLocation (Variables|/Game/Actor/AI/AIC_Enemy_Base.AIC_Enemy_Base_C|GetAttackTarget _asaic_enemy_base)) (Transformation|GetActorLocation))))))))
    (:Is%20Not%20Valid
      (Development|PrintString "Target Is None"))))

(fn GetIdealRange
  (return 1.5e+02 3e+02))

(fn GetPatrolRoute
  ;[1 1 1] PatrolRoute를 Map에서 설정된 경로로 깔아줘야함
  (return (Variables|AI|GetPatrolRoute)))

(fn SetMovementSpeed
  (params (Speed :type E_MovementSpeed%20Enum :default "NewEnumerator0"))
  (bind _output_get (Variables|/Script/Engine.CharacterMovementComponent|SetMaxWalkSpeed (Variables|Character|GetCharacterMovement) (Utilities|Select :Index Speed :NewEnumerator0 0.0 :NewEnumerator1 2e+02 :NewEnumerator2 3e+02 :NewEnumerator3 5e+02)))
  (return _output_get))