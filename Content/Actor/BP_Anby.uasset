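; Anby player character Blueprint: handles lock-on combat with parry, evade, target marking and camera view switching.
; Timelines drive parry camera blends, a dash to the target followed by a half-circle turn with quaternion slerp, and evades read from controller direction inputs.
; Only back evade moves the actor; left and right just set AnimInstance state.
; Number keys provide debug tests for Drake AI state, noise and damage senses.
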(event Custom|DynamicMoving
  (Utilities|IsValid (Variables|Default|GetMyTarget)
    (:Is%20Valid
      (DynamicAttack|DynamicMovingSetting)
      (bind _duration (Timeline|Moving PlayFromStart)
        (:Update
          (DynamicAttack|DynamicMovingMove _duration))
        (:Finished
          (Variables|Default|SetPrevCharacterLoc (Transformation|GetActorLocation))
          (Variables|Default|SetPrevCharacterQuat (Math|Conversions|ToQuaternion(Rotator) (Transformation|GetActorRotation)))
          (Variables|Default|SetTargetQuat (Math|Conversions|ToQuaternion(Rotator) (Math|Rotator|GetRotationXVector (Math|Conversions|RotationFromXVector (Math|Vector|Normalize (- (Variables|Default|GetPrevCharacterLoc) (Variables|Default|GetTargetLocation)))))))
          (bind _duration_2 (Timeline|Circle PlayFromStart)
            (:Update
              (DynamicAttack|DynamicMovingTurn _duration_2)
              (DynamicAttack|DynamicMovingRotation _duration_2))))))
    (:Is%20Not%20Valid
      (Development|PrintString "TargetIsNone"))))

(event Custom|SetTargetMarking
  ;[1 1 1 1 25] Marking
  ;;[1 1 1] 이미 마크 부착되어있으면 생성 안하도록
  (if (not (Variables|Default|GetbIsSetTargetMark))
    (Development|PrintString "Try Add mark")
    (bind _asbp_drake (Utilities|Casting|CastToBP_Drake (Variables|Default|GetMyTarget)))
    (Default|AddMarking _asbp_drake)
    (Variables|Default|SetbIsSetTargetMark true)))

(event Custom|EvadeLeft
  (Variables|/Script/WorkTest.AnbyAnimInstance|SetAnimState (Class|Anby|GetAnbyAnimInstance) "Evade_Left"))

(event Custom|EvadeBack
  (Variables|/Script/WorkTest.AnbyAnimInstance|SetAnimState (Class|Anby|GetAnbyAnimInstance) "Evade_Back"))

(event Custom|EvadeRight
  (Variables|/Script/WorkTest.AnbyAnimInstance|SetAnimState (Class|Anby|GetAnbyAnimInstance) "Evade_Right"))

(event Custom|BP_ActiveWeapon_1
  ;[1 1 1] WeaponActive
  (Animation|Montage|PlayMontage (Variables|Character|GetMesh) "/Game/Model/NewAnim/WeaponOnOff/WeaponOn_Montage.WeaponOn_Montage"))

(event Custom|BP_DisActiveWeapon_1
  ;[1 1 1] WeaponActive
  (Animation|Montage|PlayMontage (Variables|Character|GetMesh) "/Game/Model/NewAnim/WeaponOnOff/WeaponOff_Montage.WeaponOff_Montage"))

(event Custom|BP_ResetTarget_1
  ;[1 1 1 1 25] Marking
  (bind _asbp_drake (Utilities|Casting|CastToBP_Drake (Variables|Default|GetMyTarget)))
  (Default|RemoveMarking _asbp_drake false)
  (Variables|Default|SetbIsSetTargetMark false))

(event Custom|BP_Evade_1
  (bind _newtrack_0 (Timeline|ActorTurn PlayFromStart)
    (:Update
      ;[0.323 1 0 1 25] Evade
      (CallFunction|SetActorDirection _newtrack_0)
      (bind _asbp_anby_controller (Utilities|Casting|CastToBP_AnbyController (Game|GetPlayerController 0)))
      ;[1 1 1] Back / Right-Left 구분
      (if (== (Variables|/Script/WorkTest.AnbyController|GetDirectionRight _asbp_anby_controller) 0.0)
        ;[1 1 1] Ture : Back
        (if (== (Variables|/Script/WorkTest.AnbyController|GetDirectionFront _asbp_anby_controller) -1.0)
          (CallFunction|EvadeBack)
          (CallFunction|SetEvadeMoving "NewEnumerator0" 5e+02)
          (bind _alpha (Timeline|EvadeMove_Back PlayFromStart)
            (:Update
              (CallFunction|EvadeMoving _alpha)))
          (else
            (Development|PrintString "아무것도 안하기")))
        (else
          ;[1 1 1] True : Left
          (if (== (Variables|/Script/WorkTest.AnbyController|GetDirectionRight _asbp_anby_controller) -1.0)
            (CallFunction|EvadeLeft)
            (else
              ;[1 1 1] True:Right
              (if (== (Variables|/Script/WorkTest.AnbyController|GetDirectionRight _asbp_anby_controller) 1.0)
                (CallFunction|EvadeRight)
                (else
                  (Development|PrintString "아무것도 안하기"))))))))))

(event Custom|BP_Parring_1
  (bind _mytarget (Variables|Default|GetMyTarget))
  ;[1 1 1] Parring
  (Utilities|IsValid _mytarget
    (:Is%20Valid
      (bind _asbp_drake (Utilities|Casting|CastToBP_Drake _mytarget))
      (if (Variables|/Game/Actor/BP_Drake.BP_Drake_C|GetbIsCanParring _asbp_drake)
        (Development|PrintString "성공")
        (bind _ooutput (Timeline|GoParring PlayFromStart)
          (:Update
            (ParringSetting|SetCameraParringState _ooutput)
            (Camera|PlayWorldCameraShake "/Game/Actor/BP_HitCameraShake.BP_HitCameraShake_C" (Transformation|GetActorLocation) 0.0 2e+03)))
        (else
          (Development|PrintString "실패" :!label _label)
          (Timeline|GoParring PlayFromStart))))
    (:Is%20Not%20Valid
      (goto _label))))

(event EventBeginPlay
  (bind _mesh (Variables|Character|GetMesh))
  ;[1 0.9883 0 1 25] BeginPlay
  (Utilities|FlowControl|Sequence
    (:then_0
      ;[1 1 1] 멀티 상태에서 캐릭터 보이게하기
      (Components|SkeletalMesh|SetSkeletalMeshAsset _mesh "/Game/Model/SM/Anby_T-Pose.Anby_T-Pose")
      (Class|PrimitiveComponent|SetOwnerNoSee _mesh false)
      (Rendering|SetOnlyOwnerSee _mesh false :!class /Script/Engine.PrimitiveComponent)
      (Development|SetHiddeninGame _mesh false false)
      (Class|SkeletalMeshComponent|SetAnimClass _mesh "/Game/Actor/ABP_Anby.ABP_Anby_C"))
    (:then_1
      (bind _asbp_anby_controller (Utilities|Casting|CastToBP_AnbyController (Game|GetPlayerController 0)))
      (Variables|Components|SetAnby%20Controller _asbp_anby_controller)
      (bind _asbp_anby_weapon (Utilities|Casting|CastToBP_AnbyWeapon (Class|Anby|GetAnbyWeapon)))
      (Variables|Components|SetWeapon _asbp_anby_weapon))))

(event EventChangeView
  (bind _camerasystem (Variables|Default|GetCameraSystem))
  (Class|CamSettingComponent|SetPrevSetting (Variables|Default|GetCameraSystem))
  (bind _alpha (Timeline|ChangeViewTL PlayFromStart)
    (:Update
      (Class|CamSettingComponent|SetSpringArmLength _camerasystem _alpha))
    (:Finished
      (Class|CamSettingComponent|ChangeCharacterViewType _camerasystem))))

(event Input|MouseEvents|LeftMouseButton
  (params (Key :type Key%20Structure :default "None"))
  (:Pressed
    ;[1 1 1] Look at Enemy에서 Target 없으면 반환시킴
    (Utilities|IsValid (Variables|Default|GetMyTarget)
      (:Is%20Valid
        (Class|Anby|LookatEnemy)
        (CallFunction|SetTargetMarking)))))

(event Input|KeyboardEvents|G
  (params (Key :type Key%20Structure :default "None"))
  (:Pressed
    (CallFunction|DynamicMoving)))

(event Input|KeyboardEvents|SpaceBar
  (params (Key :type Key%20Structure :default "None")))

(event Input|KeyboardEvents|R
  (params (Key :type Key%20Structure :default "None"))
  ;[1 1 1] Parring
  (:Pressed
    (bind _output (Timeline|ReverseParring PlayFromStart)
      (:Update
        (ParringSetting|SetCameraNormalState _output)))))

(event Input|KeyboardEvents|1
  (params (Key :type Key%20Structure :default "None"))
  (:Pressed
    (bind _returnvalue (Actor|GetActorOfClass "/Game/Actor/BP_Drake.BP_Drake_C"))
    (bind _asaic_enemy_base (Utilities|Casting|CastToAIC_Enemy_Base (AI|GetAIController _returnvalue)))
    (Utilities|FlowControl|FlipFlop
      (:A
        (Default|SetStateasAttacking _asaic_enemy_base self)
        (Development|PrintString "AI State : Attacking"))
      (:B
        (Default|SetStateasPassive _asaic_enemy_base)
        (Development|PrintString "AI State : Passive")))))

(event Input|KeyboardEvents|2
  (params (Key :type Key%20Structure :default "None"))
  (bind _returnvalue (Transformation|GetActorLocation))
  (:Pressed
    (Class|Actor|MakeNoise 1.0 self _returnvalue 0.0 "None")
    (Effects|SpawnEmitteratLocation "/Game/Dragon_Rise/Demo/Particles/P_Explosion.P_Explosion" _returnvalue)
    (Audio|PlaySoundatLocation "/Game/Resource/Sound/Slash.Slash" _returnvalue "0, 0, 0" 1.0 1.0 0.0 0 0 0 0)))

(event Input|KeyboardEvents|3
  (params (Key :type Key%20Structure :default "None"))
  (:Pressed
    (bind _returnvalue (Actor|GetActorOfClass "/Game/Actor/BP_Drake.BP_Drake_C"))
    (Class|AISenseDamage|ReportDamageEvent _returnvalue self 1e+01 (Transformation|GetActorLocation) "0, 0, 0" "None")))

(event Input|KeyboardEvents|Z
  (params (Key :type Key%20Structure :default "None"))
  (:Pressed
    (Class|Anby|ChangeView)))

(event Input|KeyboardEvents|Escape
  (params (Key :type Key%20Structure :default "None"))
  (:Pressed
    (Game|QuitGame 0 "Quit" false)))

(fn ConstructionScript)

(fn SetCameraParringState
  (params (Alpha :type Float%20%28double-precision%29))
  (Variables|/Script/Engine.SpringArmComponent|SetTargetArmLength (Variables|Default|GetSpringArmComponent) (Math|Float|Lerp (Variables|Default|GetNormal_SpringArmLength) (Variables|Default|GetParring_SpringArmLength) Alpha))
  (Variables|/Script/Engine.SpringArmComponent|SetSocketOffset (Variables|Default|GetSpringArmComponent) (Math|Vector|Lerp(Vector) (Variables|Default|GetNormal_Offset) (Variables|Default|GetParring_Offset) Alpha))
  (Transformation|SetRelativeLocationAndRotation (Variables|Default|GetCameraComponent) (Math|Vector|Lerp(Vector) (Variables|Default|GetNormal_Loc) (Variables|Default|GetParring_Loc) Alpha) (Math|Rotator|Lerp(Rotator) (Variables|Default|GetNormal_Rot) (Variables|Default|GetParring_Rot) Alpha) false false))

(fn SetCameraNormalState
  (params (Alpha :type Float%20%28double-precision%29))
  (Variables|/Script/Engine.SpringArmComponent|SetTargetArmLength (Variables|Default|GetSpringArmComponent) (Math|Float|Lerp (Variables|Default|GetParring_SpringArmLength) (Variables|Default|GetNormal_SpringArmLength) Alpha))
  (Variables|/Script/Engine.SpringArmComponent|SetSocketOffset (Variables|Default|GetSpringArmComponent) (Math|Vector|Lerp(Vector) (Variables|Default|GetParring_Offset) (Variables|Default|GetNormal_Offset) Alpha))
  (Transformation|SetRelativeLocationAndRotation (Variables|Default|GetCameraComponent) (Math|Vector|Lerp(Vector) (Variables|Default|GetParring_Loc) (Variables|Default|GetNormal_Loc) Alpha) (Math|Rotator|Lerp(Rotator) (Variables|Default|GetParring_Rot) (Variables|Default|GetNormal_Rot) Alpha) false false))

(fn DynamicMovingSetting
  (Variables|Default|SetTargetLocation (Transformation|GetActorLocation (Variables|Default|GetMyTarget)))
  (Variables|Default|SetPrevCharacterLoc (Transformation|GetActorLocation))
  (Variables|Default|SetRadius (Math|Vector|Distance(Vector) (Class|CombatComponent|GetMoveDestination (Variables|Default|GetCombatSystem) (Variables|Default|GetTargetLocation)) (Variables|Default|GetTargetLocation))))

(fn DynamicMovingMove
  (params (alpha :type Float%20%28double-precision%29))
  (Transformation|SetActorLocation (Math|Vector|Lerp(Vector) (Variables|Default|GetPrevCharacterLoc) (Class|CombatComponent|GetMoveDestination (Variables|Default|GetCombatSystem) (Variables|Default|GetTargetLocation)) alpha) false false))

(fn DynamicMovingTurn
  (params (Alpha :type Float%20%28double-precision%29))
  (Class|CombatComponent|GetHalfCirclePosition (Variables|Default|GetCombatSystem) (Variables|Default|GetPrevCharacterLoc) (Variables|Default|GetTargetLocation) Alpha))

(fn DynamicMovingRotation
  (params (alpha :type Float%20%28double-precision%29))
  (Transformation|SetActorRotation (Class|KismetMathLibrary|QuatRotator (Class|KismetMathLibrary|QuatSlerp (Variables|Default|GetPrevCharacterQuat) (Variables|Default|GetTargetQuat) alpha))))

(fn SetActorDirection
  (params (alpha :type Float%20%28double-precision%29))
  (Transformation|SetActorRotation (Math|Interpolation|RInterpTo (Transformation|GetActorRotation) (Pawn|GetControlRotation :!class /Script/Engine.Pawn) alpha 1.0)))

(fn ChangeCameraView)

(fn SetEvadeMoving
  (params (Direction :type E_EvadeDirection%20Enum :default "NewEnumerator0") (Amount :type Float%20%28double-precision%29))
  (bind _returnvalue (Transformation|GetActorLocation))
  (bind _returnvalue_2 (Transformation|GetActorLocation))
  (bind _cameracomponent (Variables|Default|GetCameraComponent))
  (bind _cameracomponent_2 (Variables|Default|GetCameraComponent))
  (bind _returnvalue_3 (Math|Vector|GetRightVector _cameracomponent))
  (bind _returnvalue_4 (Math|Vector|GetForwardVector _cameracomponent_2))
  (bind _returnvalue_5 (- "" _returnvalue_4))
  (bind _returnvalue_6 (* _returnvalue_3 Amount))
  (bind _returnvalue_7 (* _returnvalue_5 Amount))
  (bind _returnvalue_8 (+ _returnvalue_2 _returnvalue_6))
  (bind _returnvalue_9 (+ _returnvalue _returnvalue_7))
  (switch Utilities|FlowControl|Switch|SwitchonE_EvadeDirection Direction
    (:NewEnumerator0
      (Variables|Evade|SetPrevActorLocation _returnvalue)
      (Variables|Evade|SetTargetActorLocation (Math|Vector|MakeVector (.x _returnvalue_9) (.y _returnvalue_9) (.z (Variables|Evade|GetPrevActorLocation)))))
    (:NewEnumerator2
      (Variables|Evade|SetPrevActorLocation _returnvalue_2)
      (Variables|Evade|SetTargetActorLocation (Math|Vector|MakeVector (.x _returnvalue_8) (.y _returnvalue_8) (.z (Variables|Evade|GetPrevActorLocation)))))))

(fn EvadeMoving
  (params (alpha :type Float%20%28double-precision%29))
  (Transformation|SetActorLocation (Math|Vector|Lerp(Vector) (Variables|Evade|GetPrevActorLocation) (Variables|Evade|GetTargetActorLocation) alpha) false false))

(fn SetMeshOption
  (params (isView :type Boolean))
  (Rendering|SetVisibility (Variables|Character|GetMesh) isView false))

(fn ChangeMovementState
  (params (SetParam :type Byte :default 0)))

(fn GetDirection
  (bind _anby_controller (Variables|Components|GetAnby%20Controller))
  (return (Math|Vector|MakeVector (Variables|/Script/WorkTest.AnbyController|GetDirectionFront _anby_controller) (Variables|/Script/WorkTest.AnbyController|GetDirectionRight _anby_controller) 0.0)))

(fn GetDirectionfloat
  (return 0.0))